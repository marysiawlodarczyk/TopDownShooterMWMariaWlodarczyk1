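; Player soldier pawn with world-axis movement, mouse-driven aiming, rifle firing, health and a HUD widget created on BeginPlay.
; Tick eases control yaw toward the mouse movement direction once its velocity exceeds a dead zone.
; Fire input toggles muzzle particles and sound; a muzzle-socket line trace for damage is defined but never called here.
; AnyDamage clamps damage minus health (reversed subtraction); zero sets Dead, which blocks movement, turning and firing.
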(event EventBeginPlay
  ;[0.6963 1 0.8878] HUD
  (bind _returnvalue (UserInterface|CreateWidget "/Game/UI/w_playerHUD.w_playerHUD_C" 0 self))
  (UserInterface|Viewport|AddtoViewport _returnvalue 0))

(event Collision|EventActorBeginOverlap
  (params (OtherActor :type Actor%20Object%20Reference)))

(event EventTick
  (params (DeltaSeconds :type Float%20%28single-precision%29))
  ;[1 0.8353 0.6244] rotation
  (CallFunction|UpdatePlayerLocation))

(event Game|Damage|EventAnyDamage
  (params (Damage :type Float%20%28single-precision%29) (DamageType :type Damage%20Type%20Object%20Reference) (InstigatedBy :type Controller%20Object%20Reference) (DamageCauser :type Actor%20Object%20Reference))
  ;[1 0.3955 0.4154] Damage
  (bind _output_get (CallFunction|DecreaseHealth Damage))
  (if (== _output_get 0.0)
    (Variables|Default|Setdead true)
    (CallFunction|StopFiringWeapon)))

(event Input|ActionEvents|InputActionfireweapon
  (params (Key :type Key%20Structure))
  ;[0.6935 0.95 1] fx weapon
  (:Pressed
    (CallFunction|StartFiringWeapon))
  (:Released
    (CallFunction|StopFiringWeapon)))

(event Input|AxisEvents|InputAxismoveUpDown
  (params (AxisValue :type Float%20%28single-precision%29))
  ;[0.7843 0.7095 1] movement
  (if (CallFunction|IsAlive)
    (Pawn|Input|AddMovementInput "1.000000,0.000000, 0" AxisValue false)))

(event Input|AxisEvents|InputAxismoveSide
  (params (AxisValue :type Float%20%28single-precision%29))
  ;[0.7843 0.7095 1] movement
  (if (CallFunction|IsAlive)
    (Pawn|Input|AddMovementInput "0.000000,1.000000, 0" AxisValue false)))

(fn ConstructionScript)

(fn GetMouseVelocity
  (bind _returnvalue (Game|GetPlayerController 0))
  (bind (_deltax _deltay) (Class|PlayerController|GetInputMouseDelta _returnvalue))
  (return (/ (Math|Vector2D|MakeVector2D _deltax _deltay) (Utilities|Time|GetWorldDeltaSeconds))))

(fn UpdatePlayerLocation
  (bind _returnvalue (Game|GetPlayerController 0))
  (bind _returnvalue_2 (CallFunction|GetMouseVelocity))
  (if (and (CallFunction|IsMouseAbovetheDeadZone) (CallFunction|IsAlive))
    (Pawn|SetControlRotation _returnvalue (Math|Interpolation|RInterpTo (Pawn|GetControlRotation _returnvalue :!class /Script/Engine.Controller) (Math|Rotator|MakeRotator 0.0 0.0 (Class|KismetMathLibrary|DegAtan2 (.x _returnvalue_2) (.y _returnvalue_2))) (Utilities|Time|GetWorldDeltaSeconds) (LocalVariables|Getdelta%20time%20multiply)))))

(fn IsMouseAbovetheDeadZone
  (return (> (Math|Vector2D|Vector2DLength (CallFunction|GetMouseVelocity)) (LocalVariables|Getmouse%20dead%20zone))))

(fn StartFiringWeapon
  (if (CallFunction|IsAlive)
    (Components|Activation|Activate (Variables|Default|GetP_AssaultRifle_MF) false)
    (bind _returnvalue (Audio|SpawnSound2D "/Game/Sounds/Weapon_AssaultRifle/Stereo/randomFireloop.randomFireloop" 1.0 1.0 0.0 0))
    (Variables|Default|Setweapon%20fire%20sound _returnvalue)))

(fn StopFiringWeapon
  (bind _weapon_fire_sound (Variables|Default|Getweapon%20fire%20sound))
  (Components|Activation|Deactivate (Variables|Default|GetP_AssaultRifle_MF))
  (Utilities|IsValid _weapon_fire_sound
    (:Is%20Valid
      (Audio|Components|Audio|Stop _weapon_fire_sound)
      (if (CallFunction|IsAlive)
        (Audio|SpawnSound2D "/Game/Sounds/Weapon_AssaultRifle/Stereo/gunFireEnd.gunFireEnd" 1.0 1.0 0.0 0)))))

(fn DecreaseHealth
  (params (Damage%20Amount :type Float%20%28single-precision%29))
  (bind _output_get (Variables|Default|Sethealth (Math|Float|Clamp(Float) (- Damage%20Amount (Variables|Default|Gethealth)) 0.0 1e+02)))
  (return _output_get))

(fn IsAlive
  (return (not (Variables|Default|Getdead))))

(fn WeaponTrace
  (bind _outhit (Collision|LineTraceByChannel (CallFunction|GetWeaponTraceStartLocation) (CallFunction|GetWeaponTraceEndLocation) "TraceTypeQuery1" false 0 "ForDuration"))
  (if (.bBlockingHit (Collision|BreakHitResult _outhit))
    (Game|Damage|ApplyDamage 0 (Variables|Default|Getdamage%20per%20shot) 0 0)))

(fn GetWeaponTraceStartLocation
  (return (Transformation|GetSocketLocation (Variables|Default|GetRifle) "muzzleFlashSocket")))

(fn GetWeaponTraceEndLocation
  (return (+ (* (Math|Vector|GetForwardVector (Pawn|GetControlRotation :!class /Script/Engine.Pawn)) (Variables|Default|Getwepon%20range)) (CallFunction|GetWeaponTraceStartLocation))))